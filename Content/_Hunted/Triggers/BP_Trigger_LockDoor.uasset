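; Trigger Blueprint that locks an assigned door when fired.
; Its ToTrigger override casts DoorToLock to HuntedPuzzleBase, calls LockDoor and prints the locked door's name before running the parent trigger logic.
; If the cast fails, nothing runs, including the parent call.
; The event graph holds only disabled default events.
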(event EventBeginPlay
  (|CallParentFunction) ; This node is disabled and will not be called.\nDrag off pins to build functionality.
)

(event Collision|EventActorBeginOverlap
  (params (OtherActor :type Actor%20Object%20Reference))
  (|CallParentFunction OtherActor) ; This node is disabled and will not be called.\nDrag off pins to build functionality.
)

(event EventTick
  (params (DeltaSeconds :type Float%20%28single-precision%29))
  (|CallParentFunction DeltaSeconds) ; This node is disabled and will not be called.\nDrag off pins to build functionality.
)

(fn ConstructionScript
  (|CallParentFunction))

(fn ToTrigger
  (bind _doortolock (Variables|Default|GetDoorToLock))
  (bind _ashunted_puzzle_base (Utilities|Casting|CastToHuntedPuzzleBase _doortolock))
  (Default|LockDoor _ashunted_puzzle_base)
  (Development|PrintString (Utilities|String|Append "Locked: " (Utilities|GetDisplayName _doortolock)))
  (|CallParentFunction))