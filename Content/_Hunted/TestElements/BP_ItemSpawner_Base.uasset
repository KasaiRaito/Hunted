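; BP_ItemSpawner_Base is an item spawner that labels itself with ItemName and spawns ItemToSpawn at its own transform on BeginPlay.
; Tick spins the spawned item in yaw at RotSpeed while its reference is valid.
; Once the reference is invalid, Tick calls SpawnItem, which spawns a replacement after a short Delay and stores its rotation for the spin.
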(event Custom|SpawnItem
  (Utilities|FlowControl|Delay 2.0)
  (bind _returnvalue (Game|SpawnActorfromClass (Variables|Default|GetItemToSpawn) (Transformation|GetActorTransform) "Undefined" "MultiplyWithRoot" self 0))
  (bind _output_get (Variables|Default|SetItemSpawnedReference _returnvalue))
  (Variables|Default|SetSavedRot (Transformation|GetActorRotation _output_get)))

(event Custom|Rotate
  (params (DT :type Float%20%28double-precision%29))
  (bind _output_get (Variables|Default|SetSavedRot (Math|Rotator|CombineRotators (Variables|Default|GetSavedRot) (Math|Rotator|MakeRotator 0.0 0.0 (* DT (Variables|Default|GetRotSpeed))))))
  (Transformation|SetActorRotation (Variables|Default|GetItemSpawnedReference) _output_get))

(event EventBeginPlay
  (Rendering|Components|TextRender|SetText (Variables|Default|GetName) (Variables|Default|GetItemName))
  (bind _returnvalue (Game|SpawnActorfromClass (Variables|Default|GetItemToSpawn) (Transformation|GetActorTransform) "Undefined" "MultiplyWithRoot" self 0))
  (Variables|Default|SetItemSpawnedReference _returnvalue))

(event Collision|EventActorBeginOverlap
  (params (OtherActor :type Actor%20Object%20Reference)))

(event EventTick
  (params (DeltaSeconds :type Float%20%28single-precision%29))
  (if (Utilities|IsValid (Variables|Default|GetItemSpawnedReference))
    (CallFunction|Rotate DeltaSeconds)
    (else
      (CallFunction|SpawnITem))))

(fn ConstructionScript)