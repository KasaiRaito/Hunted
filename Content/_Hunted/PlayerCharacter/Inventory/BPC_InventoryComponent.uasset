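; BPC_InventoryComponent is a player inventory component that holds an item array and opens the inventory screen.
; On BeginPlay it creates a W_Inventory_Grid widget, sizes Items to InventorySize, and passes itself to the widget's UpdateInventory.
; The IA_Inventory input adds the grid to the viewport if absent, shows the mouse cursor, and switches to UI-only input.
; It contains no logic for closing the inventory.
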(event Input|EnhancedActionEvents|EnhancedInputActionIA_Inventory
  (params (ActionValue :type Boolean) (ElapsedSeconds :type Float%20%28double-precision%29) (TriggeredSeconds :type Float%20%28double-precision%29) (InputAction :type Input%20Action%20Object%20Reference :default "/Game/_Hunted/PlayerCharacter/Inputs/Actions/Interact/IA_Inventory.IA_Inventory"))
  (bind _returnvalue (Game|GetPlayerController 0))
  (bind _inventoryreference (Variables|Default|GetInventoryReference))
  (if (not (UserInterface|Viewport|IsinViewport (Variables|Default|GetInventoryReference)))
    (UserInterface|Viewport|AddtoViewport (Variables|Default|GetInventoryReference) 0)
    (Variables|/Script/Engine.PlayerController|SetbShowMouseCursor _returnvalue true)
    (Input|SetInputModeUIOnly _returnvalue _inventoryreference "DoNotLock" false)
    (Variables|/Script/UMG.UserWidget|SetbIsFocusable _inventoryreference true)))

(event EventBeginPlay
  (bind _returnvalue (UserInterface|CreateWidget "/Game/_Hunted/PlayerCharacter/Inventory/Elements/W_Inventory_Grid.W_Inventory_Grid_C"))
  (Variables|Default|SetInventoryReference _returnvalue)
  (Utilities|Array|Resize (Variables|Default|GetItems) (Variables|Default|GetInventorySize))
  (Default|UpdateInventory (Variables|Default|GetInventoryReference) self))

(event EventTick
  (params (DeltaSeconds :type Float%20%28single-precision%29)))