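; Gameplay ability in which an enemy zombie grabs and bites the player through a paired animation.
; On activation it binds the zombie as primary and the first player as secondary to the CAS_ZombieBite Contextual Anim Scene, then starts it.
; After a short delay, if PushedZombie is false, it calls FaillPush on the zombie and ends the ability.
; This graph neither sets PushedZombie nor ends the ability when it is true.
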(event Ability|EventActivateAbility
  (bind _outbindings (Class|ContextualAnimUtilities|CreateContextualAnimSceneBindingsforTwoActors "/Game/_Hunted/Animations/CAS_ZombieBite.CAS_ZombieBite" (Class|ContextualAnimUtilities|SceneBindingContextMakefromActor (Class|HuntedEnemyGameplayAbility|GetEnemyCharacterfromActorInfo)) (Class|ContextualAnimUtilities|SceneBindingContextMakefromActor (Game|GetPlayerCharacter 0))))
  (bind _returnvalue (Class|ContextualAnimSceneActorComponent|StartContextualAnimScene (Variables|Default|GetContextualAnimSceneAcotr) _outbindings))
  (Development|PrintString (Utilities|String|ToString(Boolean) _returnvalue))
  (Utilities|FlowControl|Delay 2.0)
  (if (not (Variables|Default|GetPushedZombie))
    (bind _asbp_zombie_enemy (Utilities|Casting|CastToBP_Zombie_Enemy (Class|HuntedEnemyGameplayAbility|GetEnemyCharacterfromActorInfo)))
    (Default|FaillPush _asbp_zombie_enemy)
    (Ability|EndAbility)))

(event Ability|EventOnEndAbility
  (params (bWasCancelled :type Boolean)))