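; Base enemy character Blueprint for a zombie enemy, handling its death and the outcome of its grab attack on the player.
; On death it freezes animation, disables capsule collision, and runs timelines that sink the mesh while animating dynamic material parameters, then destroys the equipped weapon and itself.
; Push functions branch montage sections on both enemy and player to Exit or Bite, with a resettable success flag.
; Capsule hits print debug text.
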(event OnComponentHit(CapsuleComponent)
  (params (HitComponent :type Primitive%20Component%20Object%20Reference) (OtherActor :type Actor%20Object%20Reference) (OtherComp :type Primitive%20Component%20Object%20Reference) (NormalImpulse :type Vector :default "0, 0, 0") (Hit :type Hit%20Result%20Structure%20%28by%20ref%29))
  (Development|PrintString (Utilities|GetDisplayName OtherComp) true true "(R=0.317423,G=0.012803,B=1.000000,A=1.000000)" 2e+01))

(event EventBeginPlay)

(event Collision|EventActorBeginOverlap
  (params (OtherActor :type Actor%20Object%20Reference)))

(event EventTick
  (params (DeltaSeconds :type Float%20%28single-precision%29)))

(event EventOnEnemyDeath
  (bind _enemycombatcomponent (Variables|Default|GetEnemyCombatComponent))
  (bind _mesh (Variables|Character|GetMesh))
  (bind _returnvalue (Class|PawnCombatComponent|GetCharacterCurrentEquippedWeapon _enemycombatcomponent))
  (bind _returnvalue_2 (Transformation|GetWorldLocation _mesh))
  (Utilities|FlowControl|Sequence
    (:then_0
      (Variables|/Script/Engine.SkeletalMeshComponent|SetbPauseAnims (Variables|Character|GetMesh) true))
    (:then_1
      (Collision|SetCollisionEnabled (Variables|Default|GetCapsuleComponent) "NoCollision"))
    (:then_2
      (bind _returnvalue_3 (Rendering|Material|CreateDynamicMaterialInstance _mesh 0 0 "None" :!class /Script/Engine.PrimitiveComponent))
      (Variables|Default|SetDMI _returnvalue_3)
      (Variables|Default|SetStart _returnvalue_2)
      (Variables|Default|SetEnd (+ _returnvalue_2 "0.000000,0.000000,-200.000000"))
      (Utilities|FlowControl|Sequence
        (:then_0
          (bind _newtrack_0 (Timeline|Timeline PlayFromStart)
            (:Update
              (Transformation|SetWorldLocation (Variables|Character|GetMesh) (Math|Vector|Lerp(Vector) (Variables|Default|GetStart) (Variables|Default|GetEnd) _newtrack_0) false false))
            (:Finished
              (Utilities|IsValid _returnvalue
                (:Is%20Valid
                  (Actor|DestroyActor _returnvalue))
                (:Is%20Not%20Valid
                  _))
              (Actor|DestroyActor))))
        (:then_1
          (bind _newtrack_0_2 (Timeline|Timeline_0 PlayFromStart)
            (:Update
              (Rendering|Material|SetScalarParameterValue (Variables|Default|GetDMI) "Lenght" (Math|Float|Lerp 0.0 (Variables|Default|GetLengh) _newtrack_0_2) :!class /Script/Engine.MaterialInstanceDynamic))))
        (:then_2
          (bind _newtrack_0_3 (Timeline|Timeline_1 PlayFromStart)
            (:Update
              (Rendering|Material|SetScalarParameterValue (Variables|Default|GetDMI) "Intensity" (Math|Float|Lerp 0.0 (Variables|Default|GetIntensity) _newtrack_0_3) :!class /Script/Engine.MaterialInstanceDynamic))))
        (:then_3
          (bind _newtrack_0_4 (Timeline|Timeline_2 PlayFromStart)
            (:Update
              (Rendering|Material|SetScalarParameterValue (Variables|Default|GetDMI) "ShadowMask" (Math|Float|Lerp 0.0 (Variables|Default|GetShadowMask) _newtrack_0_4) :!class /Script/Engine.MaterialInstanceDynamic))))))))

(fn ConstructionScript)

(fn SuccesPush
  (Utilities|FlowControl|Sequence
    (:then_0
      (Variables|Default|SetPushZombie true))
    (:then_1
      (Class|AnimInstance|MontageSetNextSection (Components|SkeletalMesh|GetAnimInstance (Variables|Character|GetMesh)) "Loop" "Exit" "/Game/_Hunted/EnemyCharacter/EnemyZombie/Montages/QuickEvent/AM_ZombieAttack_Attacker.AM_ZombieAttack_Attacker"))
    (:then_2
      (Class|AnimInstance|MontageSetNextSection (Components|SkeletalMesh|GetAnimInstance (Variables|/Script/Engine.Character|GetMesh (Game|GetPlayerCharacter 0))) "Loop" "Exit" "/Game/_Hunted/EnemyCharacter/EnemyZombie/Montages/QuickEvent/AM_ZombieAttack_Attacker.AM_ZombieAttack_Attacker"))
    (:then_3
      (Development|PrintString "PUSH"))))

(fn FaillPush
  (Utilities|FlowControl|Sequence
    (:then_0
      (Class|AnimInstance|MontageSetNextSection (Components|SkeletalMesh|GetAnimInstance (Variables|Character|GetMesh)) "Loop" "Bite" "/Game/_Hunted/EnemyCharacter/EnemyZombie/Montages/QuickEvent/AM_ZombieAttack_Attacker.AM_ZombieAttack_Attacker"))
    (:then_1
      (Class|AnimInstance|MontageSetNextSection (Components|SkeletalMesh|GetAnimInstance (Variables|/Script/Engine.Character|GetMesh (Game|GetPlayerCharacter 0))) "Loop" "Bite" "/Game/_Hunted/PlayerCharacter/Montages/QuickEvent/AM_BitteAttemt_Victim.AM_BitteAttemt_Victim"))))

(fn ResetPush
  (Variables|Default|SetPushZombie false))